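; BP_Outline is an actor that displays a configurable static mesh and can toggle an outline on it.
; BeginPlay assigns the mesh, and CreateOutline spawns a second component with that mesh, passing the original's world transform as its relative transform.
; That copy gets a dynamic M_OutLineInst material driven by Color and Scale parameters.
; A HasOutLine flag prevents duplicates, and DeleteOutline destroys the copy and clears it.
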(event Custom|CreateOutline
  (if (not (Variables|Default|GetHasOutLine))
    (bind _returnvalue (AddComponent|AddStaticMeshComponent false (Transformation|GetWorldTransform (Variables|Default|GetStaticMesh))))
    (bind _output_get (Variables|Default|SetMeshComponent _returnvalue))
    (Components|StaticMesh|SetStaticMesh _output_get (Variables|Default|GetMesh))
    (bind _returnvalue_2 (Rendering|Material|CreateDynamicMaterialInstance _output_get 0 "/Game/Seonjae/Blueprint/M_OutLineInst.M_OutLineInst" "None" :!class /Script/Engine.PrimitiveComponent))
    (Rendering|Material|SetVectorParameterValue _returnvalue_2 "Color" (Variables|Default|GetColor) :!class /Script/Engine.MaterialInstanceDynamic)
    (Rendering|Material|SetScalarParameterValue _returnvalue_2 "Scale" (Variables|Default|GetScale) :!class /Script/Engine.MaterialInstanceDynamic)
    (Variables|Default|SetHasOutLine true)))

(event Custom|DeleteOutline
  (bind _meshcomponent (Variables|Default|GetMeshComponent))
  (Utilities|IsValid _meshcomponent
    (:Is%20Valid
      (Components|DestroyComponent _meshcomponent)
      (Variables|Default|SetHasOutLine false))))

(event EventBeginPlay
  (Components|StaticMesh|SetStaticMesh (Variables|Default|GetStaticMesh) (Variables|Default|GetMesh)))

(event Collision|EventActorBeginOverlap
  (params (OtherActor :type Actor%20Object%20Reference)))

(event EventTick
  (params (DeltaSeconds :type Float%20%28single-precision%29)))

(fn ConstructionScript)